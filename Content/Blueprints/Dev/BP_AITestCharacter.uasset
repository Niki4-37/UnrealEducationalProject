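; BP_AITestCharacter is a development test AI character that ragdolls when killed.
; BeginPlay initializes its BPAIHealthComponent with a fixed health value and binds to that component's OnDead event.
; The death handler makes the capsule ignore Pawn and WorldDynamic channels, enables mesh physics, and applies force along the shot direction at the given bone.
; An unconnected health debug print remains in the graph.
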(event Custom|OnDeath
  (params (ShotFromDirection :type Vector) (BoneName :type Name))
  (bind _capsulecomponent (Variables|Collision|GetCapsuleComponent))
  (bind _mesh (Variables|Character|GetMesh))
  (Collision|SetCollisionResponsetoChannel _capsulecomponent "ECC_Pawn" "ECR_Ignore")
  (Collision|SetCollisionResponsetoChannel _capsulecomponent "ECC_WorldDynamic" "ECR_Ignore")
  (Collision|SetCollisionEnabled _mesh "QueryAndPhysics")
  (Physics|SetSimulatePhysics _mesh true)
  (Physics|AddForce (Variables|Character|GetMesh) (* ShotFromDirection 1e+03) BoneName false))

(event EventBeginPlay
  (Default|InitHealth (Variables|Default|GetBP_AIHealthComponent) 20)
  (EventDispatchers|BindEventtoOnDead (Variables|Default|GetBP_AIHealthComponent) (EventDispatchers|CreateEvent :!event Custom|OnDeath)))

(event Collision|EventActorBeginOverlap
  (params (OtherActor :type Actor%20Object%20Reference)))

(event EventTick
  (params (DeltaSeconds :type Float%20%28single-precision%29)))

(fn ConstructionScript)