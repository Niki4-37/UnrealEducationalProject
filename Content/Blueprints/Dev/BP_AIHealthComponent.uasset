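; Health component for AI actors that tracks integer health and signals death from point damage.
; On BeginPlay it binds to the owner's point damage event, subtracting truncated damage, clamped between zero and max, and printing the result.
; At zero it unbinds and fires OnDead with shot direction and bone name.
; An any-damage handler exists, but its binding is disconnected and it never fires OnDead.
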(event EventBeginPlay
  (EventDispatchers|BindEventtoOnTakePointDamage (Components|GetOwner) (EventDispatchers|CreateEvent :!event TakePointDamage)))

(fn InitHealth
  (params (MaxHealth :type Integer))
  (bind _output_get (Variables|Default|SetMaxHealth MaxHealth))
  (Variables|Default|SetHealth _output_get))

(fn DecreaseHealth
  (params (Damage :type Integer))
  (bind _output_get (Variables|Default|SetHealth (Math|Integer|Clamp(Integer) (- (Variables|Default|GetHealth) Damage) 0 (Variables|Default|GetMaxHealth))))
  (return _output_get))

(fn TakePointDamage
  (params (DamagedActor :type Actor%20Object%20Reference) (Damage :type Float%20%28single-precision%29) (InstigatedBy :type Controller%20Object%20Reference) (HitLocation :type Vector) (FHitComponent :type Primitive%20Component%20Object%20Reference) (BoneName :type Name) (ShotFromDirection :type Vector) (DamageType :type Damage%20Type%20Object%20Reference) (DamageCauser :type Actor%20Object%20Reference))
  (bind _currenthealth (HealthAI|DecreaseHealth (Math|Float|Truncate Damage)))
  (Development|PrintString (Utilities|String|ToString(Integer) _currenthealth))
  (if (== _currenthealth 0)
    (EventDispatchers|UnbindEventfromOnTakePointDamage (Components|GetOwner) (EventDispatchers|CreateEvent :!event TakePointDamage))
    (Default|CallOnDead ShotFromDirection BoneName)))

(fn IdDead
  (return (== (Variables|Default|GetHealth) 0)))

(fn OnTakeAnyDamage
  (params (DamagedActor :type Actor%20Object%20Reference) (Damage :type Float%20%28single-precision%29) (DamageType :type Damage%20Type%20Object%20Reference) (InstigatedBy :type Controller%20Object%20Reference) (DamageCauser :type Actor%20Object%20Reference))
  (bind _currenthealth (HealthAI|DecreaseHealth (Math|Float|Truncate Damage)))
  (if (== _currenthealth 0)
    (EventDispatchers|UnbindEventfromOnTakeAnyDamage (Components|GetOwner) (EventDispatchers|CreateEvent :!event OnTakeAnyDamage))))