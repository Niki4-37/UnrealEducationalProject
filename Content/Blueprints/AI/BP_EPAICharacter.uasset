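; BP_EPAICharacter is an AI character Blueprint that displays its current health on a HealthText component.
; Tick calls ShowHealth every frame and writes the value to the text.
; ShowHealth casts the HealthComponent's owner to EPAICharacter and rebuilds absolute health as health percent times MaxHealth, returning zero if the cast fails.
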(event EventBeginPlay)

(event Collision|EventActorBeginOverlap
  (params (OtherActor :type Actor%20Object%20Reference)))

(event EventTick
  (params (DeltaSeconds :type Float%20%28single-precision%29))
  (bind _health (CallFunction|ShowHealth))
  (Rendering|Components|TextRender|SetText (Variables|Default|GetHealthText) (Utilities|Text|ToText(Float) _health "HalfToEven")))

(fn ConstructionScript)

(fn ShowHealth
  (bind _asepaicharacter (Utilities|Casting|CastToEPAICharacter (Components|GetOwner (Variables|Default|GetHealthComponent)))
    (:then
      (return (* (Class|EPHealthComponent|GetHealthPercent (Variables|/Script/EducationalProject.EPAICharacter|GetHealthComponent _asepaicharacter)) (Variables|/Script/EducationalProject.EPHealthComponent|GetMaxHealth (Variables|/Script/EducationalProject.EPAICharacter|GetHealthComponent _asepaicharacter)))))
    (:CastFailed
      (return 0.0))))